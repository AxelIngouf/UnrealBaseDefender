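; BP_Shop is the shop actor in BaseDefender, signalling breaks between waves and hosting the shop UI.
; It binds to the SpawnerManager's wave-state event to show its point light and beam only while IsOnBreak is true.
; ToggleShop creates or removes the shop window, nested in the player's HealthWidget canvas, and switches input between UI-only and game-only.
; ToggleShop itself does not check the wave state.
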(event Custom|WaveStateChange_Event
  (bind _spawnermanager (Variables|Default|GetSpawnerManager))
  (bind _bisonbreak (Variables|/Script/BaseDefender.SpawnerManager|GetbIsOnBreak _spawnermanager))
  (Rendering|SetVisibility (Variables|Default|GetPointLight) _bisonbreak false)
  (Rendering|SetVisibility (Variables|Default|GetP_ShopBeam) _bisonbreak false))

(event EventBeginPlay
  (bind _returnvalue (Actor|GetActorOfClass "/Script/BaseDefender.SpawnerManager"))
  (bind _output_get (Variables|Default|SetSpawnerManager _returnvalue))
  (EventDispatchers|BindEventtoOnWaveStateChange _output_get (delegate Custom|WaveStateChange_Event)))

(fn ConstructionScript)

(fn ToggleShop
  (Variables|Default|GetShopWindow
    (:then
      (Widget|RemovefromParent (Variables|Default|GetShopWindow))
      (Variables|Default|SetShopWindow 0)
      (Input|SetInputModeGameOnly (Game|GetPlayerController 0)))
    (:else
      (bind _returnvalue (UserInterface|CreateWidget "/Game/BaseDefender/UI/Shop/Widget_ShopWindow.Widget_ShopWindow_C" (Game|GetPlayerController 0) self))
      (Variables|Default|SetShopWindow _returnvalue)
      (bind _asbp_player (Utilities|Casting|CastToBP_Player (Game|Player|GetPlayerPawn 0)))
      (bind _returnvalue_2 (Class|CanvasPanel|AddChildtoCanvas (Variables|/Game/BaseDefender/UI/HUD/Widget_PlayerHUD.Widget_PlayerHUD_C|GetCanvasPanel_0 (Variables|/Game/BaseDefender/Characters/BP_Player.BP_Player_C|GetHealthWidget _asbp_player)) (Variables|Default|GetShopWindow)))
      (Class|CanvasPanelSlot|SetAutoSize _returnvalue_2 true)
      (Class|CanvasPanelSlot|SetAlignment _returnvalue_2 "(X=0.500000,Y=0.500000)")
      (Class|CanvasPanelSlot|SetAnchors _returnvalue_2 (LocalVariables|GetAnchorType))
      (Input|SetInputModeUIOnly (Game|GetPlayerController 0) (Variables|Default|GetShopWindow) "LockAlways"))))