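; Game mode for Base Defender that handles match audio, starting music on BeginPlay and binding to player-death, game-end and trap-destroyed events.
; Its sound functions play a random death cry, a random lose cry, or a positional, attenuated trap-destroyed sound.
; A PlayerDead flag limits the death cry to one play and suppresses the lose cry afterward, which is also skipped when Won is set.
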(event EventBeginPlay
  (EventDispatchers|BindEventtoOnPlayerDeath (EventDispatchers|CreateEvent :!event PlayDeathSound))
  (EventDispatchers|BindEventtoOnGameEnd (EventDispatchers|CreateEvent :!event PlayLoseSound))
  (EventDispatchers|BindEventtoOnTrapDestroyed (EventDispatchers|CreateEvent :!event PlayTrapDestroyedSound))
  (Audio|PlaySound2D (Variables|Default|GetMusic) 1.0 1.0 0.0 0 0))

(fn ConstructionScript)

(fn PlayTrapDestroyedSound
  (params (TrapLocation :type Vector))
  (Audio|PlaySoundatLocation "/Game/BaseDefender/Audio/S_TrapDestroyed.S_TrapDestroyed" TrapLocation "0, 0, 0" 1.0 1.0 0.0 "/Game/BaseDefender/Audio/SoundAttenuation.SoundAttenuation" 0 0))

(fn PlayLoseSound
  (if (not (Variables|Default|GetPlayerDead))
    (if (not (Variables|Default|GetbWon))
      (switch int (Math|Random|RandomInteger 4)
        (:0
          (Audio|PlaySound2D "/Game/Assets/HumanVocalizations/HumanMaleB/Wavs/voice_male_b_cry_high_04.voice_male_b_cry_high_04" 1.0 1.0 0.0 0 0))
        (:1
          (Audio|PlaySound2D "/Game/Assets/HumanVocalizations/HumanMaleB/Wavs/voice_male_b_cry_high_03.voice_male_b_cry_high_03" 1.0 1.0 0.0 0 0))
        (:2
          (Audio|PlaySound2D "/Game/Assets/HumanVocalizations/HumanMaleB/Wavs/voice_male_b_cry_high_01.voice_male_b_cry_high_01" 1.0 1.0 0.0 0 0))
        (:3
          (Audio|PlaySound2D "/Game/Assets/HumanVocalizations/HumanMaleB/Wavs/voice_male_b_cry_whimper_high_01.voice_male_b_cry_whimper_high_01" 1.0 1.0 0.0 0 0))))))

(fn PlayDeathSound
  (if (not (Variables|Default|GetPlayerDead))
    (switch int (Math|Random|RandomInteger 4)
      (:Default
        _)
      (:0
        (Audio|PlaySound2D "/Game/Assets/HumanVocalizations/HumanMaleB/Wavs/voice_male_b_death_low_10.voice_male_b_death_low_10" 1.0 1.0 0.0 0 0))
      (:1
        (Audio|PlaySound2D "/Game/Assets/HumanVocalizations/HumanMaleB/Wavs/voice_male_b_death_torture_13.voice_male_b_death_torture_13" 1.0 1.0 0.0 0 0))
      (:2
        (Audio|PlaySound2D "/Game/Assets/HumanVocalizations/HumanMaleB/Wavs/voice_male_b_death_low_01.voice_male_b_death_low_01" 1.0 1.0 0.0 0 0))
      (:3
        (Audio|PlaySound2D "/Game/Assets/HumanVocalizations/HumanMaleB/Wavs/voice_male_b_death_low_02.voice_male_b_death_low_02" 1.0 1.0 0.0 0 0)))
    (Variables|Default|SetPlayerDead true)))