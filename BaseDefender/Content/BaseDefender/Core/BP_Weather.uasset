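; Weather controller that runs the day-night cycle, rain and thunderstorms by driving the level's directional light, skylight and sky sphere.
; A looping timer oscillates sun height, flipping the sky at each extreme and mapping height to brightness unless raining.
; Timers alternate rain sound and player-attached particles, with flags for constant rain or night.
; A self-rescheduling thunder timer plays random sounds during rain, flickering the lights through chained short timers.
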(event EventBeginPlay
  (CallFunction|InitLight)
  (Utilities|Time|SetTimerbyFunctionName 0 "SimulateDay" 0.03 true)
  (bind _returnvalue (Audio|SpawnSound2D "/Game/BaseDefender/Audio/S_RainHeavy.S_RainHeavy" 0.5 1.0 0.0 0 false false))
  (bind _output_get (Variables|Default|SetRainSound _returnvalue))
  (Audio|Components|Audio|Stop _output_get)
  (CallFunction|Thunder)
  (if (Variables|Default|GetConstantRain)
    (CallFunction|StartRain)
    (else
      (Utilities|Time|SetTimerbyFunctionName 0 "StartRain" 45.0))))

(fn ConstructionScript)

(fn StartRain
  (bind _asbp_player (Utilities|Casting|CastToBP_Player (Game|Player|GetPlayerPawn 0)))
  (bind _returnvalue (Effects|SpawnEmitterAttached "/Game/Assets/Rain/Content/SoulCity/Effects/Particles/Water/P_RainStorm.P_RainStorm" (Variables|/Script/Engine.Character|GetMesh _asbp_player) "None" "360.000000,360.000000, 0" "0,180.000000, 0"))
  (Variables|Default|SetRainParticle _returnvalue)
  (Audio|Components|Audio|Play (Variables|Default|GetRainSound) 0.0)
  (if (Variables|Default|GetConstantRain)
    _
    (else
      (Utilities|Time|SetTimerbyFunctionName 0 "StopRain" 45.0)))
  (Variables|Default|SetRaining true)
  (CallFunction|SetWorldBrightness (Variables|Default|GetRainBrigthness)))

(fn StopRain
  (Components|DestroyComponent (Variables|Default|GetRainParticle))
  (Audio|Components|Audio|StopDelayed (Variables|Default|GetRainSound) 0.2)
  (Utilities|Time|SetTimerbyFunctionName 0 "StartRain" 45.0)
  (Variables|Default|SetRaining false))

(fn SimulateDay
  (bind _worldskysphere (Variables|Components|GetWorldSkySphere))
  (bind _worldskysphere_2 (Variables|Components|GetWorldSkySphere))
  (bind _sunspeed (Variables|Default|GetSunSpeed))
  (if (Variables|Default|GetConstantNight)
    (CallFunction|SetWorldBrightness (Variables|Default|GetRainBrigthness))
    (Variables|/Engine/EngineSky/BP_Sky_Sphere.BP_Sky_Sphere_C|SetSun%20height _worldskysphere -1.0)
    (Default|RefreshMaterial _worldskysphere)
    (else
      (LocalVariables|SetCurrentSunHeight (Variables|/Engine/EngineSky/BP_Sky_Sphere.BP_Sky_Sphere_C|GetSun%20height (Variables|Components|GetWorldSkySphere)))
      (if (Variables|Default|GetSunRising)
        (bind _output_get (LocalVariables|SetCurrentSunHeight (+ (LocalVariables|GetCurrentSunHeight) _sunspeed)))
        (if (>= _output_get 1.0)
          (Variables|Default|SetSunRising (not (Variables|Default|GetSunRising)) :!label _label)
          (Class|Actor|AddActorWorldRotation _worldskysphere_2 (Math|Rotator|MakeRotator 0.0 0.0 1.8e+02)))
        (else
          (bind _output_get_2 (LocalVariables|SetCurrentSunHeight (- (LocalVariables|GetCurrentSunHeight) _sunspeed)))
          (if (<= _output_get_2 -1.0)
            (goto _label)
            (else
              _))))
      (Variables|/Engine/EngineSky/BP_Sky_Sphere.BP_Sky_Sphere_C|SetSun%20height _worldskysphere_2 (LocalVariables|GetCurrentSunHeight))
      (Default|RefreshMaterial _worldskysphere_2)
      (if (not (Variables|Default|GetRaining))
        (CallFunction|SetWorldBrightness (Math|Float|MapRangeClamped (LocalVariables|GetCurrentSunHeight) -0.1 1.0 0.05 0.4))))))

(fn Thunder
  (if (Variables|Default|GetRaining)
    (switch int (Math|Random|RandomInteger 2)
      (:Default
        _)
      (:0
        (Audio|PlaySound2D "/Game/BaseDefender/Audio/thunder3.thunder3" 1.0 1.0 0.0 0 0)
        (Utilities|Time|SetTimerbyFunctionName 0 "StopThunderLight" 0.4 :!label _label)
        (CallFunction|ThunderLight))
      (:1
        (Audio|PlaySound2D "/Game/BaseDefender/Audio/thundr04.thundr04" 1.0 1.0 0.0 0 0)
        (goto _label))))
  (Utilities|Time|SetTimerbyFunctionName 0 "Thunder" (Math|Random|RandomFloatinRange 8.0 25.0)))

(fn ThunderLight
  (CallFunction|SetWorldBrightness 8.0))

(fn StopThunderLight
  (if (== (Variables|Default|GetFlashNumber) 3)
    (CallFunction|SetWorldBrightness (Variables|Default|GetRainBrigthness))
    (Variables|Default|SetFlashNumber 0)
    (else
      (CallFunction|SetWorldBrightness (Math|Random|RandomFloatinRange 1.0 (- 2.0 (* (Math|Conversions|ToFloat(Integer) (Math|Integer|%(Integer) (Variables|Default|GetFlashNumber) 2)) 2.0))))
      (Utilities|Time|SetTimerbyFunctionName 0 "StopThunderLight" 0.1)
      (Variables|Default|SetFlashNumber (+ (Variables|Default|GetFlashNumber) 1)))))

(fn SetWorldBrightness
  (params (Brightness :type Float%20%28single-precision%29))
  (Rendering|Components|Light|SetIntensity (Variables|Default|GetWorldLightComponent) Brightness)
  (Rendering|Components|Light|SetIntensity (Variables|Default|GetWorldSkyLight) (Math|Float|Max(Float) (* 3 Brightness) 1.0)))

(fn InitLight
  (bind _returnvalue (Actor|GetActorOfClass "/Script/Engine.SkyLight"))
  (Variables|Default|SetWorldSkyLight (Variables|/Script/Engine.SkyLight|GetLightComponent _returnvalue))
  (bind _returnvalue_2 (Actor|GetActorOfClass "/Script/Engine.DirectionalLight"))
  (Variables|Default|SetWorldLightComponent (Variables|/Script/Engine.Light|GetLightComponent _returnvalue_2))
  (bind _returnvalue_3 (Actor|GetActorOfClass "/Engine/EngineSky/BP_Sky_Sphere.BP_Sky_Sphere_C"))
  (Variables|Components|SetWorldSkySphere _returnvalue_3))