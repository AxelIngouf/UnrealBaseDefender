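; Player character Blueprint for BaseDefender, handling UI and audiovisual feedback for combat, traps and the shop.
; BeginPlay creates the HUD and hidden end-game widget, then binds delegates for damage, shop and trap events.
; Handlers flash a red material on damage, play trap sounds, toggle shops, and helper functions refresh trap UI and swap weapon visibility.
; An overlap volume reveals nearby enemy health bars, and Pause input toggles a lazily created menu.
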(event OnComponentBeginOverlap(EnemyHealthDisplayCollision)
  (params (OverlappedComponent :type Primitive%20Component%20Object%20Reference) (OtherActor :type Actor%20Object%20Reference) (OtherComp :type Primitive%20Component%20Object%20Reference) (OtherBodyIndex :type Integer) (bFromSweep :type Boolean) (SweepResult :type Hit%20Result%20Structure%20%28by%20ref%29))
  (bind _asbp_enemy (Utilities|Casting|CastToBP_Enemy OtherActor))
  (Rendering|SetVisibility (Variables|/Game/BaseDefender/Characters/BP_Enemy.BP_Enemy_C|GetEnnemyHealthUI _asbp_enemy) true false))

(event OnComponentEndOverlap(EnemyHealthDisplayCollision)
  (params (OverlappedComponent :type Primitive%20Component%20Object%20Reference) (OtherActor :type Actor%20Object%20Reference) (OtherComp :type Primitive%20Component%20Object%20Reference) (OtherBodyIndex :type Integer))
  (bind _asbp_enemy (Utilities|Casting|CastToBP_Enemy OtherActor))
  (Rendering|SetVisibility (Variables|/Game/BaseDefender/Characters/BP_Enemy.BP_Enemy_C|GetEnnemyHealthUI _asbp_enemy) false false))

(event Custom|OnShopOpened_Event
  (params (Shop :type Shop%20Object%20Reference))
  (bind _asbp_shop (Utilities|Casting|CastToBP_Shop Shop))
  (Default|ToggleShop _asbp_shop))

(event Custom|OnDamaged_Event
  (Rendering|Material|SetMaterial (Variables|Character|GetMesh) 0 "/Game/Assets/AssetPackProject/Content/ModularRPGHeroesPolyart/Textures/PolyArtMaskBaseTex_Mat_Red.PolyArtMaskBaseTex_Mat_Red")
  (Utilities|Time|SetTimerbyFunctionName 0 "StopDamageMaterial" 0.3))

(event Custom|OnTrapPlaced_Event
  (params (TrapPosition :type Vector))
  (Audio|PlaySoundatLocation "/Game/BaseDefender/Audio/S_PlaceTrap.S_PlaceTrap" TrapPosition "0, 0, 0" 1.0 1.0 0.0 0 0 0))

(event EventBeginPlay
  (EventDispatchers|BindEventtoOnHoldingTrap (EventDispatchers|CreateEvent :!event ChangeWeapon))
  (EventDispatchers|BindEventtoOnShopOpened (delegate Custom|OnShopOpened_Event))
  (EventDispatchers|BindEventtoOnTrapIndexChanged (EventDispatchers|CreateEvent :!event ChangeTrapUI))
  (EventDispatchers|BindEventtoOnTrapAmountChanged (EventDispatchers|CreateEvent :!event ChangeAmountTrapUI))
  (bind _returnvalue (UserInterface|CreateWidget "/Game/BaseDefender/UI/HUD/Widget_PlayerHUD.Widget_PlayerHUD_C"))
  (bind _output_get (Variables|Default|SetHealthWidget _returnvalue))
  (UserInterface|Viewport|AddtoViewport _output_get 0)
  (Variables|/Game/BaseDefender/UI/HUD/Widget_PlayerHUD.Widget_PlayerHUD_C|SetCurrentTrapIndex (Variables|Default|GetHealthWidget) 0)
  (EventDispatchers|AssignOnDamaged (delegate Custom|OnDamaged_Event))
  (bind _returnvalue_2 (UserInterface|CreateWidget "/Game/BaseDefender/UI/Menus/Widget_GameEnd.Widget_GameEnd_C"))
  (bind _output_get_2 (Variables|Default|SetEndGame _returnvalue_2))
  (UserInterface|Viewport|AddtoViewport _output_get_2 0)
  (Widget|SetVisibility (Variables|Default|GetEndGame) "Hidden")
  (EventDispatchers|AssignOnTrapPlaced (delegate Custom|OnTrapPlaced_Event)))

(event Input|ActionEvents|InputActionPause
  (params (Key :type Key%20Structure))
  (:Pressed
    (if (Variables|Default|GetIsPaused)
      (CallFunction|UnpauseGame)
      (else
        (CallFunction|PauseGame)))))

(fn ConstructionScript)

(fn ChangeTrapUI
  (Default|UpdateTrapPlaceholder (Variables|Default|GetHealthWidget) (Class|BaseDefenderCharacter|GetTrapIndex)))

(fn ChangeAmountTrapUI
  (Default|UpdateAmountTraps (Variables|Default|GetHealthWidget)))

(fn StopDamageMaterial
  (Rendering|Material|SetMaterial (Variables|Character|GetMesh) 0 "/Game/Assets/AssetPackProject/Content/ModularRPGHeroesPolyart/Textures/PolyArtMaskBaseTex_Mat.PolyArtMaskBaseTex_Mat"))

(fn PauseGame
  (bind _returnvalue (Game|GetPlayerController 0))
  (bind _output_get (Variables|Default|SetIsPaused true))
  (Game|SetGamePaused _output_get)
  (Utilities|IsValid (Variables|Default|GetPauseMenu)
    (:Is%20Valid
      _)
    (:Is%20Not%20Valid
      (bind _returnvalue_2 (UserInterface|CreateWidget "/Game/BaseDefender/UI/Menus/Widget_Pause.Widget_Pause_C" _returnvalue))
      (bind _output_get_2 (Variables|Default|SetPauseMenu _returnvalue_2))))
  (UserInterface|Viewport|AddtoViewport _output_get_2 0)
  (Input|SetInputModeGameandUI _returnvalue (Variables|Default|GetPauseMenu) "DoNotLock" true)
  (Variables|/Script/Engine.PlayerController|SetbShowMouseCursor _returnvalue true))

(fn UnpauseGame
  (bind _returnvalue (Game|GetPlayerController 0))
  (bind _output_get (Variables|Default|SetIsPaused false))
  (Game|SetGamePaused _output_get)
  (Widget|RemovefromParent (Variables|Default|GetPauseMenu))
  (Input|SetInputModeGameOnly _returnvalue)
  (Variables|/Script/Engine.PlayerController|SetbShowMouseCursor _returnvalue false))

(fn ChangeWeapon
  (params (HoldingTrap :type Boolean))
  (bind _weapon (Variables|Default|GetWeapon))
  (if (Math|Boolean|NotEqual(Boolean) HoldingTrap (Variables|Default|GetHoldingTrapLocal))
    (if HoldingTrap
      (Rendering|SetVisibility _weapon false false)
      (Audio|PlaySound2D "/Game/BaseDefender/Audio/S_EquipWeapon.S_EquipWeapon" 1.0 1.2 0.0 0 0)
      (else
        (Rendering|SetVisibility _weapon true false)
        (Audio|PlaySound2D "/Game/BaseDefender/Audio/S_EquipWeapon.S_EquipWeapon" 1.0 1.0 0.0 0 0)))
    (Variables|Default|SetHoldingTrapLocal (not (Variables|Default|GetHoldingTrapLocal)))))