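; Dwarf enemy Blueprint for melee attacks, damage feedback and death cleanup.
; Animation Blueprint events toggle the weapon's overlap collision, which damages non-Ennemy actors, and attack end turns the enemy toward the player.
; Taking damage briefly swaps the mesh material and spawns blood particles whose collisions leave random-frame splatter decals.
; EnemyDie destroys weapon, capsule, arrow and health UI components, occasionally playing a laugh.
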(event OnComponentBeginOverlap(WeaponCollision)
  (params (OverlappedComponent :type Primitive%20Component%20Object%20Reference) (OtherActor :type Actor%20Object%20Reference) (OtherComp :type Primitive%20Component%20Object%20Reference) (OtherBodyIndex :type Integer) (bFromSweep :type Boolean) (SweepResult :type Hit%20Result%20Structure%20%28by%20ref%29))
  ;[1 1 1] Weapon collision
  (if (not (Utilities|ClassIsChildOf (Utilities|GetClass OtherActor) "/Script/BaseDefender.Ennemy"))
    (Game|Damage|ApplyDamage OtherActor (Variables|Default|GetPower) (Pawn|GetController) self)))

(event Custom|OnAttackBeginEvent
  (bind _weaponcollision (Variables|Default|GetWeaponCollision))
  (Utilities|IsValid _weaponcollision
    (:Is%20Valid
      (Collision|SetCollisionEnabled _weaponcollision "QueryOnly"))))

(event Custom|OnAttackEndEvent
  (bind _weaponcollision (Variables|Default|GetWeaponCollision))
  (Utilities|IsValid _weaponcollision
    (:Is%20Valid
      (Collision|SetCollisionEnabled _weaponcollision "NoCollision")
      (Class|Ennemy|RotateTowardPlayer))))

(event Custom|OnCollideEvent
  (params (EventName :type Name) (EmitterTime :type Float%20%28single-precision%29) (ParticleTime :type Integer) (Location :type Vector) (Velocity :type Vector) (Direction :type Vector) (Normal :type Vector) (BoneName :type Name) (PhysMat :type Physical%20Material%20Object%20Reference))
  ;[1 1 1] Blood Particles
  (bind _returnvalue (Rendering|Material|CreateDynamicMaterialInstance "/Game/BaseDefender/FX/Flares/M_SplatterDecals.M_SplatterDecals" "None" :!class /Script/Engine.KismetMaterialLibrary))
  (Rendering|Material|SetScalarParameterValue _returnvalue "Frame" (Math|Conversions|ToFloat(Integer) (Math|Random|RandomInteger 11)) :!class /Script/Engine.MaterialInstanceDynamic)
  (Rendering|Decal|SpawnDecalatLocation _returnvalue (Math|Conversions|ToVector(Float) (Math|Random|RandomFloatinRange 2e+01 5e+01)) Location (Math|Conversions|RotationFromXVector Normal) 1e+01))

(event Custom|OnDamage
  ;[1 1 1] Blood Particles
  (bind _returnvalue (Effects|SpawnEmitterAttached "/Game/BaseDefender/FX/Flares/P_Splatter.P_Splatter" (Variables|Character|GetMesh self) "None" "0, 0,100.000000"))
  (EventDispatchers|BindEventtoOnParticleCollide _returnvalue (delegate Custom|OnCollideEvent))
  (Rendering|Material|SetMaterial (Variables|Character|GetMesh) 0 "/Game/Assets/GladiatorAssets/Content/Characters/DwarfGrunt/Textures/T_Dwarf_Grunt_Blue_Mat_Red.T_Dwarf_Grunt_Blue_Mat_Red")
  (Utilities|Time|SetTimerbyFunctionName 0 "StopDamageMaterial" 0.2))

(event EventBeginPlay
  (Collision|SetCollisionEnabled (Variables|Default|GetWeaponCollision) "NoCollision")
  (bind _asabp_dwarf (Utilities|Casting|CastToABP_Dwarf (Components|SkeletalMesh|GetAnimInstance (Variables|Character|GetMesh))))
  (EventDispatchers|BindEventtoOnAttackBegin _asabp_dwarf (delegate Custom|OnAttackBeginEvent))
  (EventDispatchers|BindEventtoOnAttackEnd _asabp_dwarf (delegate Custom|OnAttackEndEvent))
  (bind _aswidget_enemy_ui (Utilities|Casting|CastToWidget_EnemyUI (UserInterface|GetUserWidgetObject (Variables|Default|GetEnnemyHealthUI))))
  (Variables|/Game/BaseDefender/UI/Enemy/Widget_EnemyUI.Widget_EnemyUI_C|SetEnnemy _aswidget_enemy_ui self)
  (EventDispatchers|BindEventtoOnDeath (EventDispatchers|CreateEvent :!event EnemyDie))
  ;[1 1 1] Blood Particles
  (EventDispatchers|BindEventtoOnDamaged (delegate Custom|OnDamage)))

(fn ConstructionScript)

(fn StopDamageMaterial
  (Rendering|Material|SetMaterial (Variables|Character|GetMesh) 0 "/Game/Assets/GladiatorAssets/Content/Characters/DwarfGrunt/Textures/T_Dwarf_Grunt_Blue_Mat.T_Dwarf_Grunt_Blue_Mat"))

(fn EnemyDie
  (Components|DestroyComponent (Variables|Default|GetWarHammer))
  (Components|DestroyComponent (Variables|Default|GetWeaponCollision))
  (Components|DestroyComponent (Variables|Default|GetCapsuleComponent))
  (Components|DestroyComponent (Variables|Default|GetEnnemyHealthUI))
  (Components|DestroyComponent (Variables|Default|GetEnemyArrow))
  (if (== (Math|Random|RandomInteger 10) 0)
    (Audio|PlaySound2D "/Game/Assets/HumanVocalizations/HumanMaleB/Wavs/voice_male_b_battle_laugh_01.voice_male_b_battle_laugh_01" 1.0 1.0 0.0 0 0)))